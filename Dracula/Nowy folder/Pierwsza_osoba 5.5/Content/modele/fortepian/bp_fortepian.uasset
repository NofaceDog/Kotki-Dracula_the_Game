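; Interactable piano actor that serves as the entry point to the player's piano puzzle.
; Overlap shows an interaction clue widget and outlines the mesh through custom depth, and leaving hides both.
; NewFunction opens the piano widget with a mouse cursor and UI-only input.
; Tick polls the first-person character's solved flag and, once set, destroys the Box component and latches SHUTUP to skip further checks.
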(event EventBeginPlay)

(event EventTick
  (params (DeltaSeconds :type Float%20%28single-precision%29))
  (if (not (Variables|Default|GetSHUT%20UP))
    (bind _asbp_first_person_character (Utilities|Casting|CastToBP_FirstPersonCharacter (Game|GetPlayerCharacter 0)))
    (if (Variables|/Game/FirstPerson/Blueprints/BP_FirstPersonCharacter.BP_FirstPersonCharacter_C|Getsolved%20piano%20puzzle _asbp_first_person_character)
      (Components|DestroyComponent (Variables|Default|GetBox))
      (Variables|Default|SetSHUT%20UP true))))

(event Collision|EventActorBeginOverlap
  (params (OtherActor :type Actor%20Object%20Reference))
  (bind _returnvalue (UserInterface|CreateWidget "/Game/zagadki/WB_InteractionClue.WB_InteractionClue_C"))
  (UserInterface|Viewport|AddtoViewport _returnvalue 0)
  (Widget|SetVisibility _returnvalue "Visible")
  (Rendering|SetRenderCustomDepth (Variables|Default|GetFORTEPIAN) true))

(event Collision|EventActorEndOverlap
  (params (OtherActor :type Actor%20Object%20Reference))
  (Widget|SetVisibility (stale Collision|EventActorBeginOverlap _returnvalue) "Hidden")
  (Rendering|SetRenderCustomDepth (Variables|Default|GetFORTEPIAN) false))

(event EventNewFunction
  (params (Player :type Character%20Object%20Reference))
  (bind _returnvalue (Game|GetPlayerController 0))
  (bind _returnvalue_2 (UserInterface|CreateWidget "/Game/modele/fortepian/wbp_fortepian.wbp_fortepian_C"))
  (UserInterface|Viewport|AddtoViewport _returnvalue_2 0)
  (Variables|/Script/Engine.PlayerController|SetbShowMouseCursor _returnvalue true)
  (Input|SetInputModeUIOnly _returnvalue 0 "DoNotLock" false))

(fn ConstructionScript)