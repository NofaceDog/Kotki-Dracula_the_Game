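; Bookcase door actor for a book puzzle that swings open once the puzzle is solved.
; NewFunction shows the puzzle widget while SolvedBooks is false, creating it on first use with mouse cursor and UI-only input.
; From BeginPlay, a WaitUntiTrue watches the player's blue, red and yellow placement flags, then rotates the actor and sets SolvedBooks.
; Overlap events toggle custom depth on the mesh for highlighting.
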(event EventNewFunction
  (params (Player :type Character%20Object%20Reference))
  (bind _returnvalue (Game|GetPlayerController 0))
  (bind _asbp_first_person_character (Utilities|Casting|CastToBP_FirstPersonCharacter (Game|GetPlayerCharacter 0)))
  (if (not (Variables|/Game/FirstPerson/Blueprints/BP_FirstPersonCharacter.BP_FirstPersonCharacter_C|GetSolvedBooks _asbp_first_person_character))
    (if (Variables|Default|Getadded%20to%20viewport)
      (Widget|SetVisibility (Variables|Default|GetRefBiblioteczka) "Visible")
      (else
        (bind _returnvalue_2 (UserInterface|CreateWidget "/Game/zagadki/biblioteczka/WB_zagadkaksiazki.WB_zagadkaksiazki_C" 0 0 (.AsBP%20First%20Person%20Character (Utilities|Casting|CastToBP_FirstPersonCharacter (Game|GetPlayerCharacter 0)))))
        (UserInterface|Viewport|AddtoViewport _returnvalue_2 0)
        (Variables|Default|Setadded%20to%20viewport true)
        (Variables|/Script/Engine.PlayerController|SetbShowMouseCursor _returnvalue true)
        (Input|SetInputModeUIOnly _returnvalue 0 "DoNotLock" false)))))

(event Collision|EventActorBeginOverlap
  (params (OtherActor :type Actor%20Object%20Reference))
  (Rendering|SetRenderCustomDepth (Variables|Debug|GetStaticMeshComponent) true))

(event Collision|EventActorEndOverlap
  (params (OtherActor :type Actor%20Object%20Reference))
  (Rendering|SetRenderCustomDepth (Variables|Debug|GetStaticMeshComponent) false))

(event EventBeginPlay
  (Development|PrintText "wtf dioesnt it work???")
  (bind _asbp_first_person_character (Utilities|Casting|CastToBP_FirstPersonCharacter (Game|GetPlayerCharacter 0))
    (:then
      (Utilities|WaitUntiTrue (Math|Boolean|ANDBoolean (Variables|/Game/FirstPerson/Blueprints/BP_FirstPersonCharacter.BP_FirstPersonCharacter_C|GetNIebNaMiejscu _asbp_first_person_character) (Variables|/Game/FirstPerson/Blueprints/BP_FirstPersonCharacter.BP_FirstPersonCharacter_C|GetCzerNaMiejscu _asbp_first_person_character) (Variables|/Game/FirstPerson/Blueprints/BP_FirstPersonCharacter.BP_FirstPersonCharacter_C|GetZoltNaMiejscu _asbp_first_person_character))
        (:BecameTrue
          (Transformation|SetActorRotation "0.000000,90.000000,0.000000")
          (bind _asbp_first_person_character_2 (Utilities|Casting|CastToBP_FirstPersonCharacter (Game|GetPlayerCharacter 0)))
          (Variables|/Game/FirstPerson/Blueprints/BP_FirstPersonCharacter.BP_FirstPersonCharacter_C|SetSolvedBooks _asbp_first_person_character_2 true))))
    (:CastFailed
      (Development|PrintText "blue cast failed"))))

(fn ConstructionScript)