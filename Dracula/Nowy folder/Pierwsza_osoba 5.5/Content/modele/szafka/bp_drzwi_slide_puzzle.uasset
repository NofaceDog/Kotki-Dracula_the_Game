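; Door Blueprint that opens the slide puzzle UI and moves its mesh once that puzzle is solved.
; BeginPlay waits for the player character's SlidePuzzleSolved flag, then moves the mesh to a fixed relative location.
; Overlap toggles an interaction clue widget and custom-depth rendering on the mesh.
; NewFunction, not called within this graph, shows the puzzle widget with mouse cursor and UI-only input.
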(event EventBeginPlay
  (bind _asbp_first_person_character (Utilities|Casting|CastToBP_FirstPersonCharacter (Game|GetPlayerCharacter 0)))
  (Utilities|WaitUntiTrue (Variables|/Game/FirstPerson/Blueprints/BP_FirstPersonCharacter.BP_FirstPersonCharacter_C|GetSlidePuzzleSolved _asbp_first_person_character)
    (:BecameTrue
      (Components|MoveComponentTo (Variables|Debug|GetStaticMeshComponent) "578.888889,1335.000001,510.000000" "0, 0, 0" false false 0.2 false))))

(event EventTick
  (params (DeltaSeconds :type Float%20%28single-precision%29)))

(event EventNewFunction
  (params (Player :type Character%20Object%20Reference))
  (bind _returnvalue (Game|GetPlayerController 0))
  (bind _returnvalue_2 (UserInterface|CreateWidget "/Game/modele/szafka/WBP_SlidePuzle.WBP_SlidePuzle_C"))
  (UserInterface|Viewport|AddtoViewport _returnvalue_2 0)
  (Variables|/Script/Engine.PlayerController|SetbShowMouseCursor _returnvalue true)
  (Input|SetInputModeUIOnly _returnvalue 0 "DoNotLock" false))

(event Collision|EventActorBeginOverlap
  (params (OtherActor :type Actor%20Object%20Reference))
  (bind _returnvalue (UserInterface|CreateWidget "/Game/zagadki/WB_InteractionClue.WB_InteractionClue_C"))
  (UserInterface|Viewport|AddtoViewport _returnvalue 0)
  (Widget|SetVisibility _returnvalue "Visible")
  (Rendering|SetRenderCustomDepth (Variables|Debug|GetStaticMeshComponent) true))

(event Collision|EventActorEndOverlap
  (params (OtherActor :type Actor%20Object%20Reference))
  (Widget|SetVisibility (stale Collision|EventActorBeginOverlap _returnvalue) "Hidden")
  (Rendering|SetRenderCustomDepth (Variables|Debug|GetStaticMeshComponent) false))

(fn ConstructionScript)