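; BP_Switch1 is an interactable light switch that turns a referenced spot light on and off.
; Its Interact event flips the IsLightOn flag and sets the intensity of Light1's SpotLightComponent to a fixed value or zero.
; Each toggle also prints the new light state as text.
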(event EventInteract
  (bind _light1 (Variables|Default|GetLight1))
  (bind _spotlightcomponent (Variables|/Script/Engine.SpotLight|GetSpotLightComponent _light1))
  (if (not (Variables|Default|GetIsLightOn))
    (Variables|Default|SetIsLightOn true)
    (Development|PrintText "Light on")
    (Rendering|Components|Light|SetIntensity _spotlightcomponent 31.351671)
    (else
      (Variables|Default|SetIsLightOn false)
      (Development|PrintText "Light off")
      (Rendering|Components|Light|SetIntensity _spotlightcomponent 0.0))))

(fn ConstructionScript)