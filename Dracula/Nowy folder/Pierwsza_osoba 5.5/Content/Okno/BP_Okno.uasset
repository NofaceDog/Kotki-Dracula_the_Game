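; BP_Okno is a window Blueprint that ends the game once enough keys are collected.
; CollectKey increments the key count, and OpenwindowCheck compares it against the maximum before calling Openwindow through a DoOnce.
; Openwindow adds the W_EndScreen widget to the viewport, waits briefly, then quits the game.
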(event Custom|Open%20window
  (bind _returnvalue (UserInterface|CreateWidget "/Game/Okno/W_EndScreen.W_EndScreen_C"))
  (UserInterface|Viewport|AddtoViewport _returnvalue 0)
  (Utilities|FlowControl|Delay 1.0)
  (Game|QuitGame 0 "Quit" false))

(event Custom|Collect%20Key
  (Math|Integer|IncrementInt (Variables|Default|GetCurrect%20Keys%20Collected)))

(event Custom|Open%20window%20Check
  (if (>= (Variables|Default|GetCurrect%20Keys%20Collected) (Variables|Default|GetMax%20Keys%20Collecteable))
    (Utilities|FlowControl|DoOnce false
      (:Completed
        (CallFunction|OpenWindow)))))

(fn ConstructionScript)